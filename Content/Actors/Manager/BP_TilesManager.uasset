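; BP_TilesManager holds an array of tile actors and provides lookup and highlight helpers for them.
; Tiles are fetched by 1-based position or by display name, with "Nothing" skipping the name search, and the array length is exposed.
; Range highlighting swaps the Plane material to red or back to the basic one, using the raw array index rather than the 1-based position.
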(fn ConstructionScript)

(fn GettheRightTile
  (params (Position :type Integer))
  (return (Utilities|Array|Get(acopy) (Variables|Default|GetTiles) (- Position 1))))

(fn TileLength
  (return (Utilities|Array|Length (Variables|Default|GetTiles))))

(fn FindtheRightTile
  (params (Name :type String))
  (if (not (Utilities|Enum|Equal(Enum) Name "Nothing"))
    (bind _array_element (Utilities|Array|ForEachLoopwithBreak (Variables|Default|GetTiles))
      (:LoopBody
        (if (Utilities|Enum|Equal(Enum) (Utilities|GetDisplayName _array_element) Name)
          (return _array_element))))))

(fn ColoreRengeTiles
  (params (position :type Integer))
  (Rendering|Material|SetMaterial (Variables|/Game/Actors/Tiles/BP_Tiles.BP_Tiles_C|GetPlane (Utilities|Array|Get(acopy) (Variables|Default|GetTiles) position)) 0 "/Game/Actors/Tiles/M_RedTIle.M_RedTIle"))

(fn DecoloreRengeTiles
  (params (position :type Integer))
  (Rendering|Material|SetMaterial (Variables|/Game/Actors/Tiles/BP_Tiles.BP_Tiles_C|GetPlane (Utilities|Array|Get(acopy) (Variables|Default|GetTiles) position)) 0 "/Engine/MapTemplates/Materials/BasicAsset01.BasicAsset01"))