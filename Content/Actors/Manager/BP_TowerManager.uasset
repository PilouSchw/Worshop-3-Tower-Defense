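; Tower manager for a tile-based tower defense that tracks towers by type, resolves their attacks, upgrades base towers and destroys dead ones.
; Towers hit the first occupied tile ahead: base within two, straight within five, catapult three to five away with neighbor splash.
; Kills join DeadEnemy and update tile occupancy state.
; A Check macro stops range at hard-coded row boundaries; coloring helpers maintain range highlights.
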(fn ConstructionScript)

(fn AttackBaseTower
  (bind _levelinformations (Variables|Default|GetLevelInformations))
  (bind _tilesinformations (Variables|/Game/Actors/Manager/BP_LevelManager.BP_LevelManager_C|GetTilesInformations _levelinformations))
  (bind _tiles (Variables|/Game/Actors/Manager/BP_TilesManager.BP_TilesManager_C|GetTiles _tilesinformations))
  (if (and (Utilities|Array|IsNotEmpty (Variables|Default|GetBaseTower)) (Utilities|Array|IsNotEmpty (Variables|/Game/Actors/Manager/BP_SpawnManager.BP_SpawnManager_C|GetAllEnemy (Variables|/Game/Actors/Manager/BP_LevelManager.BP_LevelManager_C|GetSpawnInformation (Variables|Default|GetLevelInformations)))))
    (for _array_element (Variables|Default|GetBaseTower)
      (Variables|/Game/Actors/Tower/BP_BaseTower.BP_BaseTower_C|SetFirstTileAttack _array_element (+ (Variables|/Game/Actors/Tower/BP_BaseTower.BP_BaseTower_C|GetPosition _array_element) 1))
      (Variables|/Game/Actors/Tower/BP_BaseTower.BP_BaseTower_C|SetSecondTileAttack _array_element (+ (Variables|/Game/Actors/Tower/BP_BaseTower.BP_BaseTower_C|GetPosition _array_element) 2))
      (bind _returnvalue (Default|Is (Variables|/Game/Actors/Tiles/BP_Tiles.BP_Tiles_C|GetAC_StateTile (Utilities|Array|Get(acopy) _tiles (Variables|/Game/Actors/Tower/BP_BaseTower.BP_BaseTower_C|GetFirstTileAttack _array_element))) "OCCUPY" "NewEnumerator2"))
      (if _returnvalue
        (for _array_element_2 (Variables|/Game/Actors/Manager/BP_SpawnManager.BP_SpawnManager_C|GetAllEnemy (Variables|/Game/Actors/Manager/BP_LevelManager.BP_LevelManager_C|GetSpawnInformation (Variables|Default|GetLevelInformations)))
          (Utilities|Check (Variables|/Game/Character/Enemy/BP_BasicEnemy.BP_BasicEnemy_C|GetOneTileForward _array_element_2)
            (:false
              (if (== (Variables|/Game/Character/Enemy/BP_BasicEnemy.BP_BasicEnemy_C|GetPosition _array_element_2) (Variables|/Game/Actors/Tiles/BP_Tiles.BP_Tiles_C|GetTilePosition (Utilities|Array|Get(acopy) _tiles (Variables|/Game/Actors/Tower/BP_BaseTower.BP_BaseTower_C|GetFirstTileAttack _array_element))))
                (bind _output_get (Variables|/Game/Character/Enemy/BP_BasicEnemy.BP_BasicEnemy_C|SetHealth _array_element_2 (- (Variables|/Game/Character/Enemy/BP_BasicEnemy.BP_BasicEnemy_C|GetHealth _array_element_2) (CallFunction|GetBaseTowerDamage))))
                (Default|UpdateBasicEnemyHealth _array_element_2)
                (Game|Damage|ApplyDamage _array_element_2 (Math|Conversions|ToFloat(Integer) (CallFunction|GetBaseTowerDamage)) 0 0 "/Script/Engine.DamageType")
                (if (<= _output_get 0.0)
                  (Utilities|Array|Add (Variables|/Game/Actors/Manager/BP_SpawnManager.BP_SpawnManager_C|GetDeadEnemy (Variables|/Game/Actors/Manager/BP_LevelManager.BP_LevelManager_C|GetSpawnInformation (Variables|Default|GetLevelInformations))) _array_element_2)
                  (Default|Change (Variables|/Game/Actors/Tiles/BP_Tiles.BP_Tiles_C|GetAC_StateTile (Utilities|Array|Get(acopy) _tiles (Variables|/Game/Actors/Tower/BP_BaseTower.BP_BaseTower_C|GetFirstTileAttack _array_element))) "OCCUPY" "NewEnumerator4"))))))
        (else
          (bind _returnvalue_2 (Default|Is (Variables|/Game/Actors/Tiles/BP_Tiles.BP_Tiles_C|GetAC_StateTile (Utilities|Array|Get(acopy) _tiles (Variables|/Game/Actors/Tower/BP_BaseTower.BP_BaseTower_C|GetSecondTileAttack _array_element))) "OCCUPY" "NewEnumerator2"))
          (if _returnvalue_2
            (for _array_element_3 (Variables|/Game/Actors/Manager/BP_SpawnManager.BP_SpawnManager_C|GetAllEnemy (Variables|/Game/Actors/Manager/BP_LevelManager.BP_LevelManager_C|GetSpawnInformation (Variables|Default|GetLevelInformations)))
              (Utilities|Check (Variables|/Game/Character/Enemy/BP_BasicEnemy.BP_BasicEnemy_C|GetTwoTileForward _array_element_3)
                (:false
                  (if (== (Variables|/Game/Character/Enemy/BP_BasicEnemy.BP_BasicEnemy_C|GetPosition _array_element_3) (Variables|/Game/Actors/Tiles/BP_Tiles.BP_Tiles_C|GetTilePosition (Utilities|Array|Get(acopy) _tiles (Variables|/Game/Actors/Tower/BP_BaseTower.BP_BaseTower_C|GetSecondTileAttack _array_element))))
                    (bind _output_get_2 (Variables|/Game/Character/Enemy/BP_BasicEnemy.BP_BasicEnemy_C|SetHealth _array_element_3 (- (Variables|/Game/Character/Enemy/BP_BasicEnemy.BP_BasicEnemy_C|GetHealth _array_element_3) (CallFunction|GetBaseTowerDamage))))
                    (Default|UpdateBasicEnemyHealth _array_element_3)
                    (Game|Damage|ApplyDamage _array_element_3 (Math|Conversions|ToFloat(Integer) (CallFunction|GetBaseTowerDamage)) 0 0 "/Script/Engine.DamageType")
                    (if (<= _output_get_2 0.0)
                      (Utilities|Array|Add (Variables|/Game/Actors/Manager/BP_SpawnManager.BP_SpawnManager_C|GetDeadEnemy (Variables|/Game/Actors/Manager/BP_LevelManager.BP_LevelManager_C|GetSpawnInformation (Variables|Default|GetLevelInformations))) _array_element_3)
                      (Default|Change (Variables|/Game/Actors/Tiles/BP_Tiles.BP_Tiles_C|GetAC_StateTile (Utilities|Array|Get(acopy) _tiles (Variables|/Game/Actors/Tower/BP_BaseTower.BP_BaseTower_C|GetSecondTileAttack _array_element))) "OCCUPY" "NewEnumerator4"))))))))))))

(fn RemoveandDestroyDeadTowerfromtheRightArray
  (params (DeadTower :type BP%20Base%20Tower%20Object%20Reference%20%28by%20ref%29))
  (bind _straighttower (Variables|Default|GetStraightTower))
  (bind _catapulttower (Variables|Default|GetCatapultTower))
  (bind _largetower (Variables|Default|GetLargeTower))
  (bind _basetower (Variables|Default|GetBaseTower))
  (CallFunction|DecoloreTileLogic)
  (Utilities|Array|RemoveItem (Variables|BP_TowerManager_C|GetAllTower (Variables|/Game/Actors/Manager/BP_LevelManager.BP_LevelManager_C|GetTowerInformation (Variables|Default|GetLevelInformations))) DeadTower)
  (if (Utilities|Array|ContainsItem _basetower DeadTower)
    (Utilities|Array|RemoveItem _basetower DeadTower)
    (CallFunction|ColoreTileLogic :!label _label)
    (Audio|PlaySound2D "/Game/SFX/Tour_cassé.Tour_cassé" 1.0 1.0 0.0 0 0)
    (Actor|DestroyActor DeadTower)
    (elif (Utilities|Array|ContainsItem _straighttower DeadTower)
      (Utilities|Array|RemoveItem _straighttower DeadTower)
      (goto _label)
      (elif (Utilities|Array|ContainsItem _catapulttower DeadTower)
        (Utilities|Array|RemoveItem _catapulttower DeadTower)
        (goto _label)
        (elif (Utilities|Array|ContainsItem _largetower DeadTower)
          (Utilities|Array|RemoveItem _largetower DeadTower)
          (goto _label))))))

(fn GetBaseTowerDamage
  (return (Variables|/Game/Actors/Tower/BP_BaseTower.BP_BaseTower_C|Getdamage (Utilities|Array|Get(acopy) (Variables|Default|GetBaseTower)))))

(fn AttackCatapultTower
  (bind _levelinformations (Variables|Default|GetLevelInformations))
  (bind _tilesinformations (Variables|/Game/Actors/Manager/BP_LevelManager.BP_LevelManager_C|GetTilesInformations _levelinformations))
  (bind _tiles (Variables|/Game/Actors/Manager/BP_TilesManager.BP_TilesManager_C|GetTiles _tilesinformations))
  (if (and (Utilities|Array|IsNotEmpty (Variables|Default|GetCatapultTower)) (Utilities|Array|IsNotEmpty (Variables|/Game/Actors/Manager/BP_SpawnManager.BP_SpawnManager_C|GetAllEnemy (Variables|/Game/Actors/Manager/BP_LevelManager.BP_LevelManager_C|GetSpawnInformation (Variables|Default|GetLevelInformations)))))
    (for _array_element (Variables|Default|GetCatapultTower)
      (bind _output_get (Variables|/Game/Actors/Tower/BP_BaseTower.BP_BaseTower_C|SetHiddenTile _array_element (+ (Variables|/Game/Actors/Tower/BP_BaseTower.BP_BaseTower_C|GetPosition _array_element) 3)))
      (Utilities|Check _output_get
        (:false
          (bind _no_attack_ (CallFunction|CatapultZoneDmg (Utilities|Array|Get(acopy) _tiles _output_get)))
          (if _no_attack_
            (bind _result (Math|Integer|IncrementInt _output_get)
              (:%20%20
                (bind _output_get_2 (Variables|/Game/Actors/Tower/BP_BaseTower.BP_BaseTower_C|SetHiddenTile _array_element _result))
                (Utilities|Check _output_get_2
                  (:false
                    (bind _no_attack__2 (CallFunction|CatapultZoneDmg (Utilities|Array|Get(acopy) _tiles _output_get_2)))
                    (if _no_attack__2
                      (bind _result_2 (Math|Integer|IncrementInt _output_get_2)
                        (:%20%20
                          (bind _output_get_3 (Variables|/Game/Actors/Tower/BP_BaseTower.BP_BaseTower_C|SetHiddenTile _array_element _result_2))
                          (Utilities|Check _output_get_3
                            (:false
                              (CallFunction|CatapultZoneDmg (Utilities|Array|Get(acopy) _tiles _output_get_3)))))))))))))))))

(fn AttackStraightTower
  (bind _levelinformations (Variables|Default|GetLevelInformations))
  (bind _tilesinformations (Variables|/Game/Actors/Manager/BP_LevelManager.BP_LevelManager_C|GetTilesInformations _levelinformations))
  (bind _tiles (Variables|/Game/Actors/Manager/BP_TilesManager.BP_TilesManager_C|GetTiles _tilesinformations))
  (if (and (Utilities|Array|IsNotEmpty (Variables|Default|GetStraightTower)) (Utilities|Array|IsNotEmpty (Variables|/Game/Actors/Manager/BP_SpawnManager.BP_SpawnManager_C|GetAllEnemy (Variables|/Game/Actors/Manager/BP_LevelManager.BP_LevelManager_C|GetSpawnInformation (Variables|Default|GetLevelInformations)))))
    (for _array_element (Variables|Default|GetStraightTower)
      (bind _output_get (Variables|/Game/Actors/Tower/BP_BaseTower.BP_BaseTower_C|SetHiddenTile _array_element (+ 1 (Variables|/Game/Actors/Tower/BP_BaseTower.BP_BaseTower_C|GetPosition _array_element))))
      (Utilities|Check _output_get
        (:false
          (bind _noattack_ (CallFunction|StraightZoneDmg (Utilities|Array|Get(acopy) (Variables|/Game/Actors/Manager/BP_TilesManager.BP_TilesManager_C|GetTiles (Variables|/Game/Actors/Manager/BP_LevelManager.BP_LevelManager_C|GetTilesInformations (Variables|Default|GetLevelInformations))) (Variables|/Game/Actors/Tower/BP_BaseTower.BP_BaseTower_C|GetHiddenTile _array_element))))
          (if _noattack_
            (bind _result (Math|Integer|IncrementInt _output_get)
              (:%20%20
                (Utilities|Check _result
                  (:false
                    (bind _noattack__2 (CallFunction|StraightZoneDmg (Utilities|Array|Get(acopy) _tiles _result)))
                    (if _noattack__2
                      (bind _result_2 (Math|Integer|IncrementInt _result)
                        (:%20%20
                          (Utilities|Check _result_2
                            (:false
                              (bind _noattack__3 (CallFunction|StraightZoneDmg (Utilities|Array|Get(acopy) _tiles _result_2)))
                              (if _noattack__3
                                (bind _result_3 (Math|Integer|IncrementInt _result_2)
                                  (:%20%20
                                    (Utilities|Check _result_3
                                      (:false
                                        (bind _noattack__4 (CallFunction|StraightZoneDmg (Utilities|Array|Get(acopy) _tiles _result_3)))
                                        (if _noattack__4
                                          (bind _result_4 (Math|Integer|IncrementInt _result_3)
                                            (:%20%20
                                              (Utilities|Check _result_4
                                                (:false
                                                  (CallFunction|StraightZoneDmg (Utilities|Array|Get(acopy) _tiles _result_4)))))))))))))))))))))))))))

(fn CatapultZoneDmg
  (params (Tile :type BP%20Tiles%20Object%20Reference))
  (bind _damage (CallFunction|GetCatapultDamage))
  (bind _damage_2 (CallFunction|GetCatapultZoneDamage))
  (bind _damage_3 (CallFunction|GetCatapultZoneDamage))
  (bind _levelinformations (Variables|Default|GetLevelInformations))
  (bind _tileposition (Variables|/Game/Actors/Tiles/BP_Tiles.BP_Tiles_C|GetTilePosition Tile))
  (bind _returnvalue (- _tileposition 1))
  (bind _returnvalue_2 (+ _tileposition 1))
  (bind _tilesinformations (Variables|/Game/Actors/Manager/BP_LevelManager.BP_LevelManager_C|GetTilesInformations _levelinformations))
  (bind _tiles (Variables|/Game/Actors/Manager/BP_TilesManager.BP_TilesManager_C|GetTiles _tilesinformations))
  (bind _output (Utilities|Array|Get(acopy) _tiles _returnvalue))
  (bind _output_2 (Utilities|Array|Get(acopy) _tiles _returnvalue_2))
  (bind _returnvalue_3 (Default|Is (Variables|/Game/Actors/Tiles/BP_Tiles.BP_Tiles_C|GetAC_StateTile Tile) "OCCUPY" "NewEnumerator2"))
  (if _returnvalue_3
    (for _array_element (Variables|/Game/Actors/Manager/BP_SpawnManager.BP_SpawnManager_C|GetAllEnemy (Variables|/Game/Actors/Manager/BP_LevelManager.BP_LevelManager_C|GetSpawnInformation (Variables|Default|GetLevelInformations)))
      (if (== (Variables|/Game/Character/Enemy/BP_BasicEnemy.BP_BasicEnemy_C|GetPosition _array_element) (Variables|/Game/Actors/Tiles/BP_Tiles.BP_Tiles_C|GetTilePosition Tile))
        (bind _output_get (Variables|/Game/Character/Enemy/BP_BasicEnemy.BP_BasicEnemy_C|SetHealth _array_element (- (Variables|/Game/Character/Enemy/BP_BasicEnemy.BP_BasicEnemy_C|GetHealth _array_element) _damage)))
        (Default|UpdateBasicEnemyHealth _array_element)
        (Game|Damage|ApplyDamage _array_element (Math|Conversions|ToFloat(Integer) _damage) 0 0 "/Script/Engine.DamageType")
        (if (<= _output_get 0)
          (Utilities|Array|Add (Variables|/Game/Actors/Manager/BP_SpawnManager.BP_SpawnManager_C|GetDeadEnemy (Variables|/Game/Actors/Manager/BP_LevelManager.BP_LevelManager_C|GetSpawnInformation (Variables|Default|GetLevelInformations))) _array_element)
          (Default|Change (Variables|/Game/Actors/Tiles/BP_Tiles.BP_Tiles_C|GetAC_StateTile Tile) "OCCUPY" "NewEnumerator4"))))
    (bind _returnvalue_4 (Default|Is (Variables|/Game/Actors/Tiles/BP_Tiles.BP_Tiles_C|GetAC_StateTile _output) "OCCUPY" "NewEnumerator2"))
    (if _returnvalue_4
      (Utilities|Check _returnvalue
        (:false
          (for _array_element_2 (Variables|/Game/Actors/Manager/BP_SpawnManager.BP_SpawnManager_C|GetAllEnemy (Variables|/Game/Actors/Manager/BP_LevelManager.BP_LevelManager_C|GetSpawnInformation (Variables|Default|GetLevelInformations)))
            (if (== (Variables|/Game/Character/Enemy/BP_BasicEnemy.BP_BasicEnemy_C|GetPosition _array_element_2) (Variables|/Game/Actors/Tiles/BP_Tiles.BP_Tiles_C|GetTilePosition _output))
              (bind _output_get_2 (Variables|/Game/Character/Enemy/BP_BasicEnemy.BP_BasicEnemy_C|SetHealth _array_element_2 (- (Variables|/Game/Character/Enemy/BP_BasicEnemy.BP_BasicEnemy_C|GetHealth _array_element_2) _damage_2)))
              (Default|UpdateBasicEnemyHealth _array_element_2)
              (Game|Damage|ApplyDamage _array_element_2 (Math|Conversions|ToFloat(Integer) _damage_2) 0 0 "/Script/Engine.DamageType")
              (if (<= _output_get_2 0)
                (Utilities|Array|Add (Variables|/Game/Actors/Manager/BP_SpawnManager.BP_SpawnManager_C|GetDeadEnemy (Variables|/Game/Actors/Manager/BP_LevelManager.BP_LevelManager_C|GetSpawnInformation (Variables|Default|GetLevelInformations))) _array_element_2)
                (Default|Change (Variables|/Game/Actors/Tiles/BP_Tiles.BP_Tiles_C|GetAC_StateTile _output) "OCCUPY" "NewEnumerator4")))))))
    (bind _returnvalue_5 (Default|Is (Variables|/Game/Actors/Tiles/BP_Tiles.BP_Tiles_C|GetAC_StateTile _output_2) "OCCUPY" "NewEnumerator2"))
    (if _returnvalue_5
      (Utilities|Check _returnvalue_2
        (:false
          (for _array_element_3 (Variables|/Game/Actors/Manager/BP_SpawnManager.BP_SpawnManager_C|GetAllEnemy (Variables|/Game/Actors/Manager/BP_LevelManager.BP_LevelManager_C|GetSpawnInformation (Variables|Default|GetLevelInformations)))
            (if (== (Variables|/Game/Character/Enemy/BP_BasicEnemy.BP_BasicEnemy_C|GetPosition _array_element_3) (Variables|/Game/Actors/Tiles/BP_Tiles.BP_Tiles_C|GetTilePosition _output_2))
              (bind _output_get_3 (Variables|/Game/Character/Enemy/BP_BasicEnemy.BP_BasicEnemy_C|SetHealth _array_element_3 (- (Variables|/Game/Character/Enemy/BP_BasicEnemy.BP_BasicEnemy_C|GetHealth _array_element_3) _damage_3)))
              (Default|UpdateBasicEnemyHealth _array_element_3)
              (Game|Damage|ApplyDamage _array_element_3 (Math|Conversions|ToFloat(Integer) _damage_3) 0 0 "/Script/Engine.DamageType")
              (if (<= _output_get_3 0)
                (Utilities|Array|Add (Variables|/Game/Actors/Manager/BP_SpawnManager.BP_SpawnManager_C|GetDeadEnemy (Variables|/Game/Actors/Manager/BP_LevelManager.BP_LevelManager_C|GetSpawnInformation (Variables|Default|GetLevelInformations))) _array_element_3)
                (Default|Change (Variables|/Game/Actors/Tiles/BP_Tiles.BP_Tiles_C|GetAC_StateTile _output_2) "OCCUPY" "NewEnumerator4"))))
          (return false)))
      (else
        (return false)))
    (else
      (return true))))

(fn StraightZoneDmg
  (params (Tile :type BP%20Tiles%20Object%20Reference))
  (bind _damage (CallFunction|GetStraigthTowerDamage))
  (bind _returnvalue (Default|Is (Variables|/Game/Actors/Tiles/BP_Tiles.BP_Tiles_C|GetAC_StateTile Tile) "OCCUPY" "NewEnumerator2"))
  (if _returnvalue
    (for _array_element (Variables|/Game/Actors/Manager/BP_SpawnManager.BP_SpawnManager_C|GetAllEnemy (Variables|/Game/Actors/Manager/BP_LevelManager.BP_LevelManager_C|GetSpawnInformation (Variables|Default|GetLevelInformations)))
      (if (== (Variables|/Game/Character/Enemy/BP_BasicEnemy.BP_BasicEnemy_C|GetPosition _array_element) (Variables|/Game/Actors/Tiles/BP_Tiles.BP_Tiles_C|GetTilePosition Tile))
        (bind _output_get (Variables|/Game/Character/Enemy/BP_BasicEnemy.BP_BasicEnemy_C|SetHealth _array_element (- (Variables|/Game/Character/Enemy/BP_BasicEnemy.BP_BasicEnemy_C|GetHealth _array_element) _damage)))
        (Default|UpdateBasicEnemyHealth _array_element)
        (Game|Damage|ApplyDamage _array_element (Math|Conversions|ToFloat(Integer) _damage) 0 0 "/Script/Engine.DamageType")
        (if (<= _output_get 0)
          (Utilities|Array|Add (Variables|/Game/Actors/Manager/BP_SpawnManager.BP_SpawnManager_C|GetDeadEnemy (Variables|/Game/Actors/Manager/BP_LevelManager.BP_LevelManager_C|GetSpawnInformation (Variables|Default|GetLevelInformations))) _array_element)
          (Default|Change (Variables|/Game/Actors/Tiles/BP_Tiles.BP_Tiles_C|GetAC_StateTile Tile) "OCCUPY" "NewEnumerator4")
          (return false))))
    (else
      (return true))))

(fn UpgradeBaseTowertoCatapultTower
  (params (Base%20Tower :type BP%20Base%20Tower%20Object%20Reference))
  (bind _staticmesh (Variables|/Game/Actors/Tower/BP_BaseTower.BP_BaseTower_C|GetStaticMesh Base%20Tower))
  (Default|DecoloreRengeTiles (Variables|/Game/Actors/Manager/BP_LevelManager.BP_LevelManager_C|GetTilesInformations (Variables|Default|GetLevelInformations)) (Variables|/Game/Actors/Tower/BP_BaseTower.BP_BaseTower_C|GetFirstTileAttack Base%20Tower))
  (Default|DecoloreRengeTiles (Variables|/Game/Actors/Manager/BP_LevelManager.BP_LevelManager_C|GetTilesInformations (Variables|Default|GetLevelInformations)) (Variables|/Game/Actors/Tower/BP_BaseTower.BP_BaseTower_C|GetSecondTileAttack Base%20Tower))
  (Components|StaticMesh|SetStaticMesh _staticmesh "/Game/FBX/Catapulte/CATAPULTE.CATAPULTE")
  (Rendering|Material|SetMaterial _staticmesh 0 "/Game/FBX/Catapulte/CATAPULTEimage_Mat.CATAPULTEimage_Mat")
  (Variables|/Game/Actors/Tower/BP_BaseTower.BP_BaseTower_C|Setdamage Base%20Tower 3)
  (Variables|/Game/Actors/Tower/BP_BaseTower.BP_BaseTower_C|Sethealth Base%20Tower (+ (Variables|/Game/Actors/Tower/BP_BaseTower.BP_BaseTower_C|Gethealth Base%20Tower) 2.0))
  (Variables|/Game/Actors/Tower/BP_BaseTower.BP_BaseTower_C|SetMaxHealth Base%20Tower 7.0)
  (Default|UpdateUI Base%20Tower)
  (Utilities|Array|RemoveItem (Variables|Default|GetBaseTower) Base%20Tower)
  (Utilities|Array|Add (Variables|Default|GetCatapultTower) Base%20Tower)
  (Audio|PlaySound2D "/Game/SFX/Amelioration.Amelioration" 1.0 1.0 0.0 0 0)
  (CallFunction|ColoreTileLogic))

(fn UpgradeBaseTowertoStraigthTower
  (params (BaseTower :type BP%20Base%20Tower%20Object%20Reference))
  (bind _staticmesh (Variables|/Game/Actors/Tower/BP_BaseTower.BP_BaseTower_C|GetStaticMesh BaseTower))
  (Components|StaticMesh|SetStaticMesh _staticmesh "/Game/FBX/Catapulte/CATAPULTE.CATAPULTE")
  (Rendering|Material|SetMaterial _staticmesh 0 "/Game/FBX/TourLoin/TOUR_LOIN_copie_Mat.TOUR_LOIN_copie_Mat")
  (Variables|/Game/Actors/Tower/BP_BaseTower.BP_BaseTower_C|Setdamage BaseTower 2)
  (Variables|/Game/Actors/Tower/BP_BaseTower.BP_BaseTower_C|SetMaxHealth BaseTower 5.0)
  (Default|UpdateUI BaseTower)
  (Utilities|Array|RemoveItem (Variables|Default|GetBaseTower) BaseTower)
  (Utilities|Array|Add (Variables|Default|GetStraightTower) BaseTower)
  (Audio|PlaySound2D "/Game/SFX/Amelioration.Amelioration" 1.0 1.0 0.0 0 0)
  (CallFunction|ColoreTileLogic))

(fn GetStraigthTowerDamage
  (return (Variables|/Game/Actors/Tower/BP_BaseTower.BP_BaseTower_C|Getdamage (Utilities|Array|Get(acopy) (Variables|Default|GetStraightTower)))))

(fn GetCatapultDamage
  (return (Variables|/Game/Actors/Tower/BP_BaseTower.BP_BaseTower_C|Getdamage (Utilities|Array|Get(acopy) (Variables|Default|GetCatapultTower)))))

(fn GetCatapultZoneDamage
  (return (- (Variables|/Game/Actors/Tower/BP_BaseTower.BP_BaseTower_C|Getdamage (Utilities|Array|Get(acopy) (Variables|Default|GetCatapultTower))) 2)))

(fn ColoreTileLogic
  (bind _levelinformations (Variables|Default|GetLevelInformations))
  (bind _levelinformations_2 (Variables|Default|GetLevelInformations))
  (bind _levelinformations_3 (Variables|Default|GetLevelInformations))
  (bind _tilesinformations (Variables|/Game/Actors/Manager/BP_LevelManager.BP_LevelManager_C|GetTilesInformations _levelinformations_2))
  (bind _tilesinformations_2 (Variables|/Game/Actors/Manager/BP_LevelManager.BP_LevelManager_C|GetTilesInformations _levelinformations_3))
  (bind _tilesinformations_3 (Variables|/Game/Actors/Manager/BP_LevelManager.BP_LevelManager_C|GetTilesInformations _levelinformations))
  (for _array_element (Variables|Default|GetCatapultTower)
    (Utilities|Check (+ (Variables|/Game/Actors/Tower/BP_BaseTower.BP_BaseTower_C|GetPosition _array_element) 1)
      (:false
        (Default|DecoloreRengeTiles _tilesinformations_3 (+ (Variables|/Game/Actors/Tower/BP_BaseTower.BP_BaseTower_C|GetPosition _array_element) 1))
        (Utilities|Check (+ (Variables|/Game/Actors/Tower/BP_BaseTower.BP_BaseTower_C|GetPosition _array_element) 2)
          (:false
            (Default|DecoloreRengeTiles _tilesinformations_3 (+ (Variables|/Game/Actors/Tower/BP_BaseTower.BP_BaseTower_C|GetPosition _array_element) 2))
            (Utilities|Check (+ (Variables|/Game/Actors/Tower/BP_BaseTower.BP_BaseTower_C|GetPosition _array_element) 3)
              (:false
                (Default|ColoreRengeTiles _tilesinformations_3 (+ (Variables|/Game/Actors/Tower/BP_BaseTower.BP_BaseTower_C|GetPosition _array_element) 3))
                (Utilities|Check (+ (Variables|/Game/Actors/Tower/BP_BaseTower.BP_BaseTower_C|GetPosition _array_element) 4)
                  (:false
                    (Default|ColoreRengeTiles _tilesinformations_3 (+ (Variables|/Game/Actors/Tower/BP_BaseTower.BP_BaseTower_C|GetPosition _array_element) 4))
                    (Utilities|Check (+ (Variables|/Game/Actors/Tower/BP_BaseTower.BP_BaseTower_C|GetPosition _array_element) 5)
                      (:false
                        (Default|ColoreRengeTiles _tilesinformations_3 (+ (Variables|/Game/Actors/Tower/BP_BaseTower.BP_BaseTower_C|GetPosition _array_element) 5)))))))))))))
  (for _array_element_2 (Variables|Default|GetStraightTower)
    (Utilities|Check (+ (Variables|/Game/Actors/Tower/BP_BaseTower.BP_BaseTower_C|GetPosition _array_element_2) 1)
      (:false
        (Default|ColoreRengeTiles _tilesinformations (+ (Variables|/Game/Actors/Tower/BP_BaseTower.BP_BaseTower_C|GetPosition _array_element_2) 1))
        (Utilities|Check (+ (Variables|/Game/Actors/Tower/BP_BaseTower.BP_BaseTower_C|GetPosition _array_element_2) 2)
          (:false
            (Default|ColoreRengeTiles _tilesinformations (+ (Variables|/Game/Actors/Tower/BP_BaseTower.BP_BaseTower_C|GetPosition _array_element_2) 2))
            (Utilities|Check (+ (Variables|/Game/Actors/Tower/BP_BaseTower.BP_BaseTower_C|GetPosition _array_element_2) 3)
              (:false
                (Default|ColoreRengeTiles _tilesinformations (+ (Variables|/Game/Actors/Tower/BP_BaseTower.BP_BaseTower_C|GetPosition _array_element_2) 3))
                (Utilities|Check (+ (Variables|/Game/Actors/Tower/BP_BaseTower.BP_BaseTower_C|GetPosition _array_element_2) 4)
                  (:false
                    (Default|ColoreRengeTiles _tilesinformations (+ (Variables|/Game/Actors/Tower/BP_BaseTower.BP_BaseTower_C|GetPosition _array_element_2) 4))
                    (Utilities|Check (+ (Variables|/Game/Actors/Tower/BP_BaseTower.BP_BaseTower_C|GetPosition _array_element_2) 5)
                      (:false
                        (Default|ColoreRengeTiles _tilesinformations (+ (Variables|/Game/Actors/Tower/BP_BaseTower.BP_BaseTower_C|GetPosition _array_element_2) 5)))))))))))))
  (for _array_element_3 (Variables|Default|GetBaseTower)
    (bind _output_get (Variables|/Game/Actors/Tower/BP_BaseTower.BP_BaseTower_C|SetFirstTileAttack _array_element_3 (+ (Variables|/Game/Actors/Tower/BP_BaseTower.BP_BaseTower_C|GetPosition _array_element_3) 1)))
    (Default|ColoreRengeTiles _tilesinformations_2 _output_get)
    (bind _output_get_2 (Variables|/Game/Actors/Tower/BP_BaseTower.BP_BaseTower_C|SetSecondTileAttack _array_element_3 (+ (Variables|/Game/Actors/Tower/BP_BaseTower.BP_BaseTower_C|GetPosition _array_element_3) 2)))
    (Default|ColoreRengeTiles _tilesinformations_2 _output_get_2)))

(fn DecoloreTileLogic
  (bind _levelinformations (Variables|Default|GetLevelInformations))
  (bind _levelinformations_2 (Variables|Default|GetLevelInformations))
  (bind _levelinformations_3 (Variables|Default|GetLevelInformations))
  (bind _tilesinformations (Variables|/Game/Actors/Manager/BP_LevelManager.BP_LevelManager_C|GetTilesInformations _levelinformations))
  (bind _tilesinformations_2 (Variables|/Game/Actors/Manager/BP_LevelManager.BP_LevelManager_C|GetTilesInformations _levelinformations_2))
  (bind _tilesinformations_3 (Variables|/Game/Actors/Manager/BP_LevelManager.BP_LevelManager_C|GetTilesInformations _levelinformations_3))
  (for _array_element (Variables|Default|GetDeadTower)
    (if (Utilities|Array|ContainsItem (Variables|Default|GetBaseTower) _array_element)
      (Utilities|Check (+ (Variables|/Game/Actors/Tower/BP_BaseTower.BP_BaseTower_C|GetPosition _array_element) 1)
        (:false
          (Default|DecoloreRengeTiles _tilesinformations (+ (Variables|/Game/Actors/Tower/BP_BaseTower.BP_BaseTower_C|GetPosition _array_element) 1))
          (Utilities|Check (+ 2 (Variables|/Game/Actors/Tower/BP_BaseTower.BP_BaseTower_C|GetPosition _array_element))
            (:false
              (Default|DecoloreRengeTiles _tilesinformations (+ 2 (Variables|/Game/Actors/Tower/BP_BaseTower.BP_BaseTower_C|GetPosition _array_element))))))))
    (if (Utilities|Array|ContainsItem (Variables|Default|GetStraightTower) _array_element)
      (Utilities|Check (+ 1 (Variables|/Game/Actors/Tower/BP_BaseTower.BP_BaseTower_C|GetPosition _array_element))
        (:false
          (Default|DecoloreRengeTiles _tilesinformations_3 (+ 1 (Variables|/Game/Actors/Tower/BP_BaseTower.BP_BaseTower_C|GetPosition _array_element)))
          (Utilities|Check (+ 2 (Variables|/Game/Actors/Tower/BP_BaseTower.BP_BaseTower_C|GetPosition _array_element))
            (:false
              (Default|DecoloreRengeTiles _tilesinformations_3 (+ 2 (Variables|/Game/Actors/Tower/BP_BaseTower.BP_BaseTower_C|GetPosition _array_element)))
              (Utilities|Check (+ 3 (Variables|/Game/Actors/Tower/BP_BaseTower.BP_BaseTower_C|GetPosition _array_element))
                (:false
                  (Default|DecoloreRengeTiles _tilesinformations_3 (+ 3 (Variables|/Game/Actors/Tower/BP_BaseTower.BP_BaseTower_C|GetPosition _array_element)))
                  (Utilities|Check (+ 4 (Variables|/Game/Actors/Tower/BP_BaseTower.BP_BaseTower_C|GetPosition _array_element))
                    (:false
                      (Default|DecoloreRengeTiles _tilesinformations_3 (+ 4 (Variables|/Game/Actors/Tower/BP_BaseTower.BP_BaseTower_C|GetPosition _array_element)))
                      (Utilities|Check (+ 5 (Variables|/Game/Actors/Tower/BP_BaseTower.BP_BaseTower_C|GetPosition _array_element))
                        (:false
                          (Default|DecoloreRengeTiles _tilesinformations_3 (+ 5 (Variables|/Game/Actors/Tower/BP_BaseTower.BP_BaseTower_C|GetPosition _array_element))))))))))))))
    (if (Utilities|Array|ContainsItem (Variables|Default|GetCatapultTower) _array_element)
      (Utilities|Check (+ 3 (Variables|/Game/Actors/Tower/BP_BaseTower.BP_BaseTower_C|GetPosition _array_element))
        (:false
          (Default|DecoloreRengeTiles _tilesinformations_2 (+ 3 (Variables|/Game/Actors/Tower/BP_BaseTower.BP_BaseTower_C|GetPosition _array_element)))
          (Utilities|Check (+ 4 (Variables|/Game/Actors/Tower/BP_BaseTower.BP_BaseTower_C|GetPosition _array_element))
            (:false
              (Default|DecoloreRengeTiles _tilesinformations_2 (+ 4 (Variables|/Game/Actors/Tower/BP_BaseTower.BP_BaseTower_C|GetPosition _array_element)))
              (Utilities|Check (+ 5 (Variables|/Game/Actors/Tower/BP_BaseTower.BP_BaseTower_C|GetPosition _array_element))
                (:false
                  (Default|DecoloreRengeTiles _tilesinformations_2 (+ 5 (Variables|/Game/Actors/Tower/BP_BaseTower.BP_BaseTower_C|GetPosition _array_element))))))))))))