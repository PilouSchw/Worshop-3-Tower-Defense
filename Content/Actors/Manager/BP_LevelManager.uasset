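; BP_LevelManager sequences the rounds of a turn-based tower defense game through player, tower and enemy phases.
; PlayerPhase starts a round only when IsNextRound is set, clearing it before TowerPhase fires Base, Catapult and Straight towers via TowerInformation.
; EnemyPhase then has SpawnInformation move or attack with Basic, Horse and Spear enemies, and returns to PlayerPhase.
; Zero-HP units are destroyed after every step; BeginPlay is empty.
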(event EventBeginPlay)

(fn ConstructionScript)

(fn PlayerPhase
  (if (Variables|Default|GetbIsNextRound?)
    (Variables|Default|SetbIsNextRound? false)
    (CallFunction|TowerPhase)))

(fn TowerPhase
  (bind _towerinformation (Variables|Default|GetTowerInformation))
  (bind _spawninformation (Variables|Default|GetSpawnInformation))
  (Default|AttackBaseTower _towerinformation)
  (Default|DestroyAllTowerandEnemyat0HP _spawninformation)
  (Default|AttackCatapultTower _towerinformation)
  (Default|DestroyAllTowerandEnemyat0HP _spawninformation)
  (Default|AttackStraightTower _towerinformation)
  (Default|DestroyAllTowerandEnemyat0HP _spawninformation)
  (CallFunction|EnemyPhase))

(fn EnemyPhase
  (bind _spawninformation (Variables|Default|GetSpawnInformation))
  (Default|MoveorAttackBasicEnemy _spawninformation)
  (Default|DestroyAllTowerandEnemyat0HP _spawninformation)
  (Default|MoveorAttackHorseEnemy _spawninformation)
  (Default|DestroyAllTowerandEnemyat0HP _spawninformation)
  (Default|MoveorAttackSpearEnemy _spawninformation)
  (Default|DestroyAllTowerandEnemyat0HP _spawninformation)
  (CallFunction|PlayerPhase))