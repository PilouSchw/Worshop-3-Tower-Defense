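; BP_RessourcesManager is a manager actor that tracks resource buildings in an overall array plus per-type Mine and Sawmill arrays.
; RemoveBuildingFromTheRightArray removes a given building from AllBuilding, then from whichever type array contains it, checking Mine before Sawmill.
; The building actor is destroyed only when it is found in one of those two type arrays.
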(fn ConstructionScript)

(fn RemoveBuildingfromtheRightArray
  (params (Ressources :type BP%20Mine%20Object%20Reference))
  (Utilities|Array|RemoveItem (Variables|Default|GetAllBuilding) Ressources)
  (if (Utilities|Array|ContainsItem (Variables|Default|GetMine) Ressources)
    (Utilities|Array|RemoveItem (Variables|Default|GetMine) Ressources)
    (Actor|DestroyActor Ressources :!label _label)
    (elif (Utilities|Array|ContainsItem (Variables|Default|GetSawmill) Ressources)
      (Utilities|Array|RemoveItem (Variables|Default|GetSawmill) Ressources)
      (goto _label))))