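; BP_Tiles is a tile actor that initializes its tile state and tracks mouse hover over its plane.
; On BeginPlay it sets the OCCUPY state on its ACStateTile component to a default enum value.
; Cursor events on the Plane set TileName to the component's display name, or to "Nothing" when the cursor leaves.
; A TilesLength helper sets TilePosition to the length of the Tiles array in the supplied TileInformation.
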(event OnBeginCursorOver(Plane)
  (params (TouchedComponent :type Primitive%20Component%20Object%20Reference))
  (Variables|Default|SetTileName (Utilities|GetDisplayName TouchedComponent)))

(event OnEndCursorOver(Plane)
  (params (TouchedComponent :type Primitive%20Component%20Object%20Reference))
  (Variables|Default|SetTileName "Nothing"))

(event EventBeginPlay
  (Default|Change (Variables|Default|GetAC_StateTile) "OCCUPY" "NewEnumerator4"))

(fn ConstructionScript)

(fn TilesLength
  (params (TileInformation :type BP%20Tiles%20Manager%20Object%20Reference))
  (Variables|Default|SetTilePosition (Utilities|Array|Length (Variables|/Game/Actors/Manager/BP_TilesManager.BP_TilesManager_C|GetTiles TileInformation))))