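; Player character for a turn-based tower defense game, handling camera-relative movement, building purchase and placement, and menus.
; Shop selections spend rocks or wood and fill inventories; clicks trace under the cursor to spawn buildings on free tiles and register them with LevelInformation.
; EnemyTurn sequences tower attacks, resource collection and enemy actions with delays, then returns control.
; HUD updates show defeat at zero health; placement preview is unwired.
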(event Custom|Move
  (params (Value :type Vector%202D%20Structure))
  (bind _returnvalue (Pawn|GetControlRotation :!class /Script/Engine.Pawn))
  (Pawn|Input|AddMovementInput (Math|Vector|GetRightVector (Math|Rotator|MakeRotator 0.0 0.0 (.yaw _returnvalue))) (.x Value) false)
  (Pawn|Input|AddMovementInput (Math|Vector|GetForwardVector (Math|Rotator|MakeRotator 0.0 0.0 (.yaw _returnvalue))) (.y Value) false))

(event Custom|Look
  (params (Value :type Vector%202D%20Structure))
  (Pawn|Input|AddControllerYawInput (.x Value))
  (Pawn|Input|AddControllerPitchInput (.y Value)))

(event Custom|Toggle%20Pause
  (if (Utilities|IsValid (Variables|UI|GetPause%20UI))
    _
    (else
      (bind _returnvalue (UserInterface|CreateWidget "/Game/UI/MenuUI/WBP_PauseMenu.WBP_PauseMenu_C"))
      (Variables|UI|SetPause%20UI _returnvalue)))
  (if (UserInterface|Viewport|IsinViewport (Variables|UI|GetPause%20UI))
    (Widget|RemovefromParent (Variables|UI|GetPause%20UI))
    (else
      (UserInterface|Viewport|AddtoViewport (Variables|UI|GetPause%20UI) 0))))

(event Custom|Select%20Or%20Place%20Building
  (if (Variables|Default|GetPlayerTurn)
    (if (not (CallFunction|InventoryEmpty?))
      (if (Utilities|Array|IsNotEmpty (Variables|Inventory|GetTower%20Inventory))
        (CallFunction|PlaceBaseTowerBuilding)
        (Audio|PlaySound2D "/Game/SFX/Tour_posé.Tour_posé" 1.0 1.0 0.0 0 0)
        (Default|ColoreTileLogic (Variables|/Game/Actors/Manager/BP_LevelManager.BP_LevelManager_C|GetTowerInformation (Variables|Default|GetLevelInformation)))
        (elif (Utilities|Array|IsNotEmpty (Variables|Inventory|GetSawmillInventory))
          (CallFunction|PlaceSawmillBuilding)
          (Audio|PlaySound2D "/Game/SFX/Scierie_posé.Scierie_posé" 1.0 1.0 0.0 0 0)
          (elif (Utilities|Array|IsNotEmpty (Variables|Inventory|GetMineInventory))
            (CallFunction|PlaceMineBuilding)
            (Audio|PlaySound2D "/Game/SFX/Mine_cassé.Mine_cassé" 1.0 1.0 0.0 0 0)))))))

(event Custom|Toggle%20Shop
  (if (Utilities|IsValid (Variables|UI|GetShop%20UI))
    _
    (else
      (bind _returnvalue (UserInterface|CreateWidget "/Game/UI/MenuUI/WBP_BuyingMenu.WBP_BuyingMenu_C"))
      (Variables|UI|SetShop%20UI _returnvalue)))
  (if (UserInterface|Viewport|IsinViewport (Variables|UI|GetShop%20UI))
    (Widget|RemovefromParent (Variables|UI|GetShop%20UI))
    (else
      (UserInterface|Viewport|AddtoViewport (Variables|UI|GetShop%20UI) 0))))

(event Custom|UpdateBaseUI
  (Default|Update (Variables|UI|GetBaseUI) (Utilities|Text|ToText(Integer) (Variables|ResourceManagement|GetRocks)) (Utilities|Text|ToText(Integer) (Variables|ResourceManagement|GetWoods)) (/ (Variables|ResourceManagement|GetHealth) 5.0))
  (if (== (Variables|ResourceManagement|GetHealth) 0.0)
    (Widget|RemovefromParent (Variables|UI|GetBaseUI))
    (bind _returnvalue (UserInterface|CreateWidget "/Game/UI/MenuUI/WBP_DefeatUI.WBP_DefeatUI_C"))
    (UserInterface|Viewport|AddtoViewport _returnvalue 0)))

(event Custom|Base%20UI
  (bind _returnvalue (UserInterface|CreateWidget "/Game/UI/MenuUI/WBP_BaseUI.WBP_BaseUI_C"))
  (Default|Update _returnvalue (Utilities|Text|ToText(Integer) (Variables|ResourceManagement|GetRocks)) (Utilities|Text|ToText(Integer) (Variables|ResourceManagement|GetWoods)) (Math|Conversions|ToFloat(Integer) (/ (Variables|ResourceManagement|GetHealth) 5)))
  (bind _output_get (Variables|UI|SetBaseUI _returnvalue))
  (UserInterface|Viewport|AddtoViewport _output_get 0))

(event Custom|EnemyTurn
  (bind _levelinformation (Variables|Default|GetLevelInformation))
  (bind _levelinformation_2 (Variables|Default|GetLevelInformation))
  (bind _spawninformation (Variables|/Game/Actors/Manager/BP_LevelManager.BP_LevelManager_C|GetSpawnInformation _levelinformation))
  (bind _towerinformation (Variables|/Game/Actors/Manager/BP_LevelManager.BP_LevelManager_C|GetTowerInformation _levelinformation_2))
  (bind _spawninformation_2 (Variables|/Game/Actors/Manager/BP_LevelManager.BP_LevelManager_C|GetSpawnInformation _levelinformation_2))
  (if (not (Variables|Default|GetPlayerTurn))
    (Default|AttackBaseTower _towerinformation)
    (Default|DestroyAllTower,EnemyandBuildingat0HP _spawninformation_2)
    (Utilities|FlowControl|Delay (Variables|Default|GetMoveOrAttackDuration))
    (Default|AttackCatapultTower _towerinformation)
    (Default|DestroyAllTower,EnemyandBuildingat0HP _spawninformation_2)
    (Utilities|FlowControl|Delay (Variables|Default|GetMoveOrAttackDuration))
    (Default|AttackStraightTower _towerinformation)
    (Default|DestroyAllTower,EnemyandBuildingat0HP _spawninformation_2)
    (Default|CollectRessourcesEachRounds (Variables|/Game/Actors/Manager/BP_LevelManager.BP_LevelManager_C|GetRessourcesInformation (Variables|Default|GetLevelInformation)))
    (Default|MoveorAttackBasicEnemy _spawninformation)
    (Default|DestroyAllTower,EnemyandBuildingat0HP _spawninformation)
    (Utilities|FlowControl|Delay (Variables|Default|GetMoveOrAttackDuration))
    (Default|MoveorAttackHorseEnemy _spawninformation)
    (Default|DestroyAllTower,EnemyandBuildingat0HP _spawninformation)
    (Utilities|FlowControl|Delay (Variables|Default|GetMoveOrAttackDuration))
    (Default|MoveorAttackSpearEnemy _spawninformation)
    (Default|DestroyAllTower,EnemyandBuildingat0HP _spawninformation)
    (Utilities|FlowControl|Delay (Variables|Default|GetMoveOrAttackDuration))
    (Variables|Default|SetPlayerTurn true)))

(event Input|EnhancedActionEvents|EnhancedInputActionIA_Look
  (params (ActionValue :type Vector%202D%20Structure) (ElapsedSeconds :type Float%20%28double-precision%29) (TriggeredSeconds :type Float%20%28double-precision%29) (InputAction :type Input%20Action%20Object%20Reference :default "/Game/ControlTemporaire/Input/IA_Look.IA_Look"))
  (CallFunction|Look ActionValue))

(event Input|EnhancedActionEvents|EnhancedInputActionIA_Move
  (params (ActionValue :type Vector%202D%20Structure) (ElapsedSeconds :type Float%20%28double-precision%29) (TriggeredSeconds :type Float%20%28double-precision%29) (InputAction :type Input%20Action%20Object%20Reference :default "/Game/ControlTemporaire/Input/IA_Move.IA_Move"))
  (CallFunction|Move ActionValue))

(event Input|EnhancedActionEvents|EnhancedInputActionIA_Pause
  (params (ActionValue :type Boolean) (ElapsedSeconds :type Float%20%28double-precision%29) (TriggeredSeconds :type Float%20%28double-precision%29) (InputAction :type Input%20Action%20Object%20Reference :default "/Game/ControlTemporaire/Input/IA_Pause.IA_Pause"))
  (:Started
    (CallFunction|TogglePause)))

(event Input|EnhancedActionEvents|EnhancedInputActionIA_Click
  (params (ActionValue :type Boolean) (ElapsedSeconds :type Float%20%28double-precision%29) (TriggeredSeconds :type Float%20%28double-precision%29) (InputAction :type Input%20Action%20Object%20Reference :default "/Game/ControlTemporaire/Input/IA_Click.IA_Click"))
  (:Started
    (CallFunction|SelectorPlaceBuilding)))

(event Input|EnhancedActionEvents|EnhancedInputActionIA_Shop
  (params (ActionValue :type Boolean) (ElapsedSeconds :type Float%20%28double-precision%29) (TriggeredSeconds :type Float%20%28double-precision%29) (InputAction :type Input%20Action%20Object%20Reference :default "/Game/ControlTemporaire/Input/IA_Shop.IA_Shop"))
  (:Started
    (CallFunction|ToggleShop)))

(event Input|EnhancedActionEvents|EnhancedInputActionIA_SecondaryAction
  (params (ActionValue :type Boolean) (ElapsedSeconds :type Float%20%28double-precision%29) (TriggeredSeconds :type Float%20%28double-precision%29) (InputAction :type Input%20Action%20Object%20Reference :default "/Game/ControlTemporaire/Input/IA_SecondaryAction.IA_SecondaryAction"))
  (:Started
    (CallFunction|ToggleUpgradeUI)))

(event EventBeginPlay
  (Variables|/Script/Engine.PlayerController|SetbShowMouseCursor (Game|GetPlayerController 0) true))

(event EventTick
  (params (DeltaSeconds :type Float%20%28single-precision%29)))

(fn ConstructionScript)

(fn SelectBaseTowerBuilding
  (bind _returnvalue (Game|GetPlayerController 0))
  (bind (_worldlocation _worlddirection) (Game|Player|ConvertMouseLocationToWorldSpace _returnvalue))
  (Utilities|Array|Clear (Variables|Inventory|GetTower%20Inventory))
  (bind _outhit (Collision|LineTraceByChannel _worldlocation (* _worlddirection (Variables|Default|GetRange)) "TraceTypeQuery2" false 0 "ForDuration"))
  (if (Actor|ActorHasTag (.HitActor (Collision|BreakHitResult _outhit)) "BaseTower")
    (Utilities|Array|Add (Variables|Inventory|GetTower%20Inventory) "/Game/Actors/Tower/BP_BaseTower.BP_BaseTower_C")))

(fn PlaceBaseTowerBuilding
  (bind _returnvalue (Game|GetPlayerController 0))
  (bind _levelinformation (Variables|Default|GetLevelInformation))
  (bind (_worldlocation _worlddirection) (Game|Player|ConvertMouseLocationToWorldSpace _returnvalue))
  (bind _towerinformation (Variables|/Game/Actors/Manager/BP_LevelManager.BP_LevelManager_C|GetTowerInformation _levelinformation))
  (bind _basetower (Variables|/Game/Actors/Manager/BP_TowerManager.BP_TowerManager_C|GetBaseTower _towerinformation))
  (bind _outhit (Collision|LineTraceByChannel _worldlocation (* _worlddirection (Variables|Default|GetRange)) "TraceTypeQuery2" false 0 "ForDuration"))
  (if (Actor|ActorHasTag (.HitActor (Collision|BreakHitResult _outhit)) "Tile")
    (bind _returnvalue_2 (Default|Is (Variables|/Game/Actors/Tiles/BP_Tiles.BP_Tiles_C|GetAC_StateTile (Default|FindtheRightTile (Variables|/Game/Actors/Manager/BP_LevelManager.BP_LevelManager_C|GetTilesInformations (Variables|Default|GetLevelInformation)) (Utilities|GetDisplayName (.HitActor (Collision|BreakHitResult _outhit))))) "OCCUPY" "NewEnumerator4"))
    (if _returnvalue_2
      (Default|Change (Variables|/Game/Actors/Tiles/BP_Tiles.BP_Tiles_C|GetAC_StateTile (Default|FindtheRightTile (Variables|/Game/Actors/Manager/BP_LevelManager.BP_LevelManager_C|GetTilesInformations (Variables|Default|GetLevelInformation)) (Utilities|GetDisplayName (.HitActor (Collision|BreakHitResult _outhit))))) "OCCUPY" "NewEnumerator1")
      (bind _returnvalue_3 (Game|SpawnActorfromClass (Utilities|Array|Get(acopy) (Variables|Inventory|GetTower%20Inventory)) (Transformation|GetActorTransform (Default|FindtheRightTile (Variables|/Game/Actors/Manager/BP_LevelManager.BP_LevelManager_C|GetTilesInformations (Variables|Default|GetLevelInformation)) (Utilities|GetDisplayName (.HitActor (Collision|BreakHitResult _outhit))))) "AlwaysSpawn" "MultiplyWithRoot" 0 0))
      (bind _returnvalue_4 (Utilities|Array|Add _basetower _returnvalue_3))
      (Utilities|Array|Add (Variables|/Game/Actors/Manager/BP_TowerManager.BP_TowerManager_C|GetAllTower _towerinformation) _returnvalue_3)
      (Variables|/Game/Actors/Tower/BP_BaseTower.BP_BaseTower_C|SetPosition (Utilities|Array|Get(acopy) _basetower _returnvalue_4) (Variables|/Game/Actors/Tiles/BP_Tiles.BP_Tiles_C|GetTilePosition (Default|FindtheRightTile (Variables|/Game/Actors/Manager/BP_LevelManager.BP_LevelManager_C|GetTilesInformations (Variables|Default|GetLevelInformation)) (Utilities|GetDisplayName (.HitActor (Collision|BreakHitResult _outhit))))))
      (CallFunction|ClearAllInventory)
      (CallFunction|UpdateBaseUI (Variables|/Game/Actors/Manager/BP_LevelManager.BP_LevelManager_C|GetPlayerInformation (Variables|Default|GetLevelInformation))))))

(fn SelectShopTowerBuilding
  (if (and (>= (Variables|ResourceManagement|GetRocks) 1) (>= (Variables|ResourceManagement|GetWoods) 1))
    (Variables|ResourceManagement|SetRocks (- (Variables|ResourceManagement|GetRocks) 1))
    (Variables|ResourceManagement|SetWoods (- (Variables|ResourceManagement|GetWoods) 1))
    (CallFunction|ClearInventory)
    (Utilities|Array|Add (Variables|Inventory|GetTower%20Inventory) "/Game/Actors/Tower/BP_BaseTower.BP_BaseTower_C")))

(fn ToggleUpgradeUI
  (bind _returnvalue (Game|GetPlayerController 0))
  (bind _returnvalue_2 (Game|GetPlayerController 0))
  (bind _basetowerupgrade (Variables|Inventory|GetBaseTowerUpgrade))
  (bind (_worldlocation _worlddirection) (Game|Player|ConvertMouseLocationToWorldSpace _returnvalue))
  (bind _outhit (Collision|LineTraceByChannel _worldlocation (* _worlddirection (Variables|Default|GetRange)) "TraceTypeQuery2" false 0 "ForDuration"))
  (if (Actor|ActorHasTag (.HitActor (Collision|BreakHitResult _outhit)) "BaseTower")
    (for _array_element (Variables|/Game/Actors/Manager/BP_TowerManager.BP_TowerManager_C|GetBaseTower (Variables|/Game/Actors/Manager/BP_LevelManager.BP_LevelManager_C|GetTowerInformation (Variables|Default|GetLevelInformation)))
      (if (Utilities|Operators|EqualEqual (Transformation|GetActorLocation _array_element) (Transformation|GetActorLocation (.HitActor (Collision|BreakHitResult _outhit))) 0.0)
        (Utilities|Array|Clear _basetowerupgrade)
        (Utilities|Array|Add _basetowerupgrade _array_element)
        (if (Utilities|IsValid (Variables|UI|GetUpgrade%20UI))
          _
          (else
            (bind _returnvalue_3 (UserInterface|CreateWidget "/Game/UI/TowerUI/WBP_UpgradeMenu.WBP_UpgradeMenu_C" (Game|GetPlayerController 0)))
            (Variables|UI|SetUpgrade%20UI _returnvalue_3)))
        (if (UserInterface|Viewport|IsinViewport (Variables|UI|GetUpgrade%20UI))
          (Widget|RemovefromParent (Variables|UI|GetUpgrade%20UI))
          (Input|SetInputModeGameOnly _returnvalue_2 false)
          (else
            (UserInterface|Viewport|AddtoViewport (Variables|UI|GetUpgrade%20UI) 0)
            (Input|SetInputModeGameandUI _returnvalue_2 (Variables|UI|GetUpgrade%20UI) "DoNotLock" true false)))))))

(fn PlaceSawmillBuilding
  (bind _returnvalue (Game|GetPlayerController 0))
  (bind _levelinformation (Variables|Default|GetLevelInformation))
  (bind (_worldlocation _worlddirection) (Game|Player|ConvertMouseLocationToWorldSpace _returnvalue))
  (bind _ressourcesinformation (Variables|/Game/Actors/Manager/BP_LevelManager.BP_LevelManager_C|GetRessourcesInformation _levelinformation))
  (bind _sawmill (Variables|/Game/Actors/Manager/BP_RessourcesManager.BP_RessourcesManager_C|GetSawmill _ressourcesinformation))
  (bind _outhit (Collision|LineTraceByChannel _worldlocation (* _worlddirection (Variables|Default|GetRange)) "TraceTypeQuery2" false 0 "ForDuration"))
  (if (Actor|ActorHasTag (.HitActor (Collision|BreakHitResult _outhit)) "Tile")
    (bind _returnvalue_2 (Default|Is (Variables|/Game/Actors/Tiles/BP_Tiles.BP_Tiles_C|GetAC_StateTile (Default|FindtheRightTile (Variables|/Game/Actors/Manager/BP_LevelManager.BP_LevelManager_C|GetTilesInformations (Variables|Default|GetLevelInformation)) (Utilities|GetDisplayName (.HitActor (Collision|BreakHitResult _outhit))))) "OCCUPY" "NewEnumerator4"))
    (if _returnvalue_2
      (Default|Change (Variables|/Game/Actors/Tiles/BP_Tiles.BP_Tiles_C|GetAC_StateTile (Default|FindtheRightTile (Variables|/Game/Actors/Manager/BP_LevelManager.BP_LevelManager_C|GetTilesInformations (Variables|Default|GetLevelInformation)) (Utilities|GetDisplayName (.HitActor (Collision|BreakHitResult _outhit))))) "OCCUPY" "NewEnumerator3")
      (bind _returnvalue_3 (Game|SpawnActorfromClass (Utilities|Array|Get(acopy) (Variables|Inventory|GetSawmillInventory)) (Transformation|GetActorTransform (Default|FindtheRightTile (Variables|/Game/Actors/Manager/BP_LevelManager.BP_LevelManager_C|GetTilesInformations (Variables|Default|GetLevelInformation)) (Utilities|GetDisplayName (.HitActor (Collision|BreakHitResult _outhit))))) "AlwaysSpawn" "MultiplyWithRoot" 0 0))
      (bind _returnvalue_4 (Utilities|Array|Add _sawmill _returnvalue_3))
      (Utilities|Array|Add (Variables|/Game/Actors/Manager/BP_RessourcesManager.BP_RessourcesManager_C|GetAllBuilding _ressourcesinformation) _returnvalue_3)
      (Variables|/Game/Actors/Ressources/BP_Mine.BP_Mine_C|SetPosition (Utilities|Array|Get(acopy) _sawmill _returnvalue_4) (Variables|/Game/Actors/Tiles/BP_Tiles.BP_Tiles_C|GetTilePosition (Default|FindtheRightTile (Variables|/Game/Actors/Manager/BP_LevelManager.BP_LevelManager_C|GetTilesInformations (Variables|Default|GetLevelInformation)) (Utilities|GetDisplayName (.HitActor (Collision|BreakHitResult _outhit))))))
      (CallFunction|ClearAllInventory)
      (CallFunction|UpdateBaseUI (Variables|/Game/Actors/Manager/BP_LevelManager.BP_LevelManager_C|GetPlayerInformation (Variables|Default|GetLevelInformation))))))

(fn PlaceMineBuilding
  (bind _returnvalue (Game|GetPlayerController 0))
  (bind _levelinformation (Variables|Default|GetLevelInformation))
  (bind (_worldlocation _worlddirection) (Game|Player|ConvertMouseLocationToWorldSpace _returnvalue))
  (bind _ressourcesinformation (Variables|/Game/Actors/Manager/BP_LevelManager.BP_LevelManager_C|GetRessourcesInformation _levelinformation))
  (bind _mine (Variables|/Game/Actors/Manager/BP_RessourcesManager.BP_RessourcesManager_C|GetMine _ressourcesinformation))
  (bind _outhit (Collision|LineTraceByChannel _worldlocation (* _worlddirection (Variables|Default|GetRange)) "TraceTypeQuery2" false 0 "ForDuration"))
  (if (Actor|ActorHasTag (.HitActor (Collision|BreakHitResult _outhit)) "Tile")
    (bind _returnvalue_2 (Default|Is (Variables|/Game/Actors/Tiles/BP_Tiles.BP_Tiles_C|GetAC_StateTile (Default|FindtheRightTile (Variables|/Game/Actors/Manager/BP_LevelManager.BP_LevelManager_C|GetTilesInformations (Variables|Default|GetLevelInformation)) (Utilities|GetDisplayName (.HitActor (Collision|BreakHitResult _outhit))))) "OCCUPY" "NewEnumerator4"))
    (if _returnvalue_2
      (Default|Change (Variables|/Game/Actors/Tiles/BP_Tiles.BP_Tiles_C|GetAC_StateTile (Default|FindtheRightTile (Variables|/Game/Actors/Manager/BP_LevelManager.BP_LevelManager_C|GetTilesInformations (Variables|Default|GetLevelInformation)) (Utilities|GetDisplayName (.HitActor (Collision|BreakHitResult _outhit))))) "OCCUPY" "NewEnumerator3")
      (bind _returnvalue_3 (Game|SpawnActorfromClass (Utilities|Array|Get(acopy) (Variables|Inventory|GetMineInventory)) (Transformation|GetActorTransform (Default|FindtheRightTile (Variables|/Game/Actors/Manager/BP_LevelManager.BP_LevelManager_C|GetTilesInformations (Variables|Default|GetLevelInformation)) (Utilities|GetDisplayName (.HitActor (Collision|BreakHitResult _outhit))))) "AlwaysSpawn" "MultiplyWithRoot" 0 0))
      (bind _returnvalue_4 (Utilities|Array|Add _mine _returnvalue_3))
      (Utilities|Array|Add (Variables|/Game/Actors/Manager/BP_RessourcesManager.BP_RessourcesManager_C|GetAllBuilding _ressourcesinformation) _returnvalue_3)
      (Variables|/Game/Actors/Ressources/BP_Mine.BP_Mine_C|SetPosition (Utilities|Array|Get(acopy) _mine _returnvalue_4) (Variables|/Game/Actors/Tiles/BP_Tiles.BP_Tiles_C|GetTilePosition (Default|FindtheRightTile (Variables|/Game/Actors/Manager/BP_LevelManager.BP_LevelManager_C|GetTilesInformations (Variables|Default|GetLevelInformation)) (Utilities|GetDisplayName (.HitActor (Collision|BreakHitResult _outhit))))))
      (CallFunction|ClearAllInventory)
      (CallFunction|UpdateBaseUI (Variables|/Game/Actors/Manager/BP_LevelManager.BP_LevelManager_C|GetPlayerInformation (Variables|Default|GetLevelInformation))))))

(fn ClearInventory
  (Utilities|Array|Clear (Variables|Inventory|GetTower%20Inventory))
  (Utilities|Array|Clear (Variables|Inventory|GetMineInventory))
  (Utilities|Array|Clear (Variables|Inventory|GetSawmillInventory)))

(fn SelectMineShop
  (if (>= (Variables|ResourceManagement|GetWoods) 1)
    (Variables|ResourceManagement|SetWoods (- (Variables|ResourceManagement|GetWoods) 1))
    (CallFunction|ClearInventory)
    (Utilities|Array|Add (Variables|Inventory|GetMineInventory) "/Game/Actors/Ressources/BP_Mine.BP_Mine_C")))

(fn SelectSawmillShop
  (if (>= (Variables|ResourceManagement|GetRocks) 1)
    (Variables|ResourceManagement|SetRocks (- (Variables|ResourceManagement|GetRocks) 1))
    (CallFunction|ClearInventory)
    (Utilities|Array|Add (Variables|Inventory|GetSawmillInventory) "/Game/Actors/Ressources/BP_Sawmill.BP_Sawmill_C")))

(fn PreviewTowerorBuildings
  (bind _returnvalue (Game|GetPlayerController 0))
  (bind (_worldlocation _worlddirection) (Game|Player|ConvertMouseLocationToWorldSpace _returnvalue))
  (bind _outhit (Collision|LineTraceByChannel _worldlocation (* _worlddirection (Variables|Default|GetRange)) "TraceTypeQuery2" false 0 "ForDuration"))
  (if (Actor|ActorHasTag (.HitActor (Collision|BreakHitResult _outhit)) "Tile")
    (return (Transformation|GetActorTransform (.HitActor (Collision|BreakHitResult _outhit))))))

(fn ClearAllInventory
  (Utilities|Array|Clear (Variables|Inventory|GetTower%20Inventory))
  (Utilities|Array|Clear (Variables|Inventory|GetMineInventory))
  (Utilities|Array|Clear (Variables|Inventory|GetSawmillInventory))
  (Components|StaticMesh|SetStaticMesh (Variables|Default|GetPreviewMesh) 0))

(fn UpdateUI)

(fn InventoryEmpty?
  (return (Math|Boolean|ANDBoolean (Utilities|Array|IsEmpty (Variables|Inventory|GetTower%20Inventory)) (Utilities|Array|IsEmpty (Variables|Inventory|GetMineInventory)) (Utilities|Array|IsEmpty (Variables|Inventory|GetSawmillInventory)))))

(fn IFGetVectors
  (bind _returnvalue (Transformation|GetActorRotation))
  (return (Math|Vector|GetUpVector _returnvalue) (Math|Vector|GetRightVector _returnvalue)))