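; BP_PlayerCharacter is a player character Blueprint that handles basic movement and camera look through Enhanced Input.
; IA_Look and IA_Move forward their values to Look and Move events, keeping the logic separate from the input bindings.
; Look drives controller yaw and pitch, while Move adds movement along right and forward vectors built from control yaw only, so view pitch does not affect direction.
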(event Custom|Look
  (params (Value :type Vector%202D%20Structure))
  (Pawn|Input|AddControllerYawInput (.x Value))
  (Pawn|Input|AddControllerPitchInput (.y Value)))

(event Custom|Move
  (params (Value :type Vector%202D%20Structure))
  (bind _returnvalue (Pawn|GetControlRotation :!class /Script/Engine.Pawn))
  (Pawn|Input|AddMovementInput (Math|Vector|GetRightVector (Math|Rotator|MakeRotator 0.0 0.0 (.yaw _returnvalue))) (.x Value) false)
  (Pawn|Input|AddMovementInput (Math|Vector|GetForwardVector (Math|Rotator|MakeRotator 0.0 0.0 (.yaw _returnvalue))) (.y Value) false))

(event Input|EnhancedActionEvents|EnhancedInputActionIA_Look
  (params (ActionValue :type Vector%202D%20Structure) (ElapsedSeconds :type Float%20%28double-precision%29) (TriggeredSeconds :type Float%20%28double-precision%29) (InputAction :type Input%20Action%20Object%20Reference :default "/Game/InputTempo/Actions/IA_Look.IA_Look"))
  (CallFunction|Look ActionValue))

(event Input|EnhancedActionEvents|EnhancedInputActionIA_Move
  (params (ActionValue :type Vector%202D%20Structure) (ElapsedSeconds :type Float%20%28double-precision%29) (TriggeredSeconds :type Float%20%28double-precision%29) (InputAction :type Input%20Action%20Object%20Reference :default "/Game/InputTempo/Actions/IA_Move.IA_Move"))
  (CallFunction|Move ActionValue))

(fn ConstructionScript)